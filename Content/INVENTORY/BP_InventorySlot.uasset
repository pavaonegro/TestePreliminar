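; Inventory slot built as a bag (Bolsa) that stores a single grabbable actor dropped into it.
; Overlapping Box_AbreFecha toggles the open state and swaps three bag materials.
; While open, CollisionDrop enlarges the bag on overlap and binds to the actor's GrabComponent grab and drop events.
; Dropping disables physics, attaches and shrinks the item relative to the bag's scale; grabbing or leaving releases it at original scale.
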(event `self.ReceiveBeginPlay`
  (set `self.InitialCellScale` (`SceneComponent.K2_GetComponentScale` (`self.Bolsa`))))

(event `self.Box_AbreFecha.OnComponentBeginOverlap`
  (params (OverlappedComponent :type "PrimitiveComponent Object Reference") (OtherActor :type "Actor Object Reference") (OtherComp :type "PrimitiveComponent Object Reference") (OtherBodyIndex :type Integer) (bFromSweep :type Boolean) (SweepResult :type "HitResult Structure (by ref)"))
  (`/Engine/EditorBlueprintResources/StandardMacros.FlipFlop`
    (:`A`
      (set `self.Aberto_OU_Fechado` true)
      (`PrimitiveComponent.SetMaterialByName` (`self.Bolsa`) "Green_Desligar" "/Game/INVENTORY/Cinto/DiscMaterial.DiscMaterial")
      (`PrimitiveComponent.SetMaterialByName` (`self.Bolsa`) "PresilhaBlack_Desligar" "/Game/INVENTORY/Cinto/DiscMaterial.DiscMaterial")
      (`PrimitiveComponent.SetMaterialByName` (`self.Bolsa`) "Corda_Desligar" "/Game/INVENTORY/Cinto/DiscMaterial.DiscMaterial"))
    (:`B`
      (set `self.Aberto_OU_Fechado` false)
      (`PrimitiveComponent.SetMaterialByName` (`self.Bolsa`) "Green_Desligar" "/Game/INVENTORY/Cinto/Green_Desligar.Green_Desligar")
      (`PrimitiveComponent.SetMaterialByName` (`self.Bolsa`) "PresilhaBlack_Desligar" "/Game/INVENTORY/Cinto/presilhablack_Desligar.presilhablack_Desligar")
      (`PrimitiveComponent.SetMaterialByName` (`self.Bolsa`) "Corda_Desligar" "/Game/INVENTORY/Cinto/Corda_Desligar.Corda_Desligar"))))

(event `self.CollisionDrop.OnComponentBeginOverlap`
  (params (OverlappedComponent :type "PrimitiveComponent Object Reference") (OtherActor :type "Actor Object Reference") (OtherComp :type "PrimitiveComponent Object Reference") (OtherBodyIndex :type Integer) (bFromSweep :type Boolean) (SweepResult :type "HitResult Structure (by ref)"))
  (if (`self.Aberto_OU_Fechado`)
    (for _array_element (`self.K2_GetComponentsByClass` OtherActor "/Game/VRTemplate/Blueprints/GrabComponent.GrabComponent_C")
      (`KismetArrayLibrary.Array_Add` (`self.TrackedGrabComponent`) _array_element)
      (add `/Game/VRTemplate/Blueprints/GrabComponent.OnGrabbed` _array_element (delegate `OnGrabbed_Event`))
      (add `/Game/VRTemplate/Blueprints/GrabComponent.OnDropped` _array_element (delegate `OnDropped_Event`)))
    (`self.IncreaseCellSize`)))

(event `OnGrabbed_Event`
  (params (SelfReference :type "/Game/VRTemplate/Blueprints/GrabComponent Object Reference"))
  (`self.TryDropObject` (`ActorComponent.GetOwner` SelfReference)))

(event `OnDropped_Event`
  (params (SelfReference :type "/Game/VRTemplate/Blueprints/GrabComponent Object Reference"))
  (`self.TryCaptureObject` SelfReference)
  (`self.DecreaseCellSize`))

(event `self.CollisionDrop.OnComponentEndOverlap`
  (params (OverlappedComponent :type "PrimitiveComponent Object Reference") (OtherActor :type "Actor Object Reference") (OtherComp :type "PrimitiveComponent Object Reference") (OtherBodyIndex :type Integer))
  (if (`self.Aberto_OU_Fechado`)
    (`self.TryDropObject` OtherActor)
    (for _array_element (`self.K2_GetComponentsByClass` OtherActor "/Game/VRTemplate/Blueprints/GrabComponent.GrabComponent_C")
      (`KismetArrayLibrary.Array_RemoveItem` (`self.TrackedGrabComponent`) _array_element)
      (remove `/Game/VRTemplate/Blueprints/GrabComponent.OnGrabbed` _array_element (delegate `OnGrabbed_Event`))
      (remove `/Game/VRTemplate/Blueprints/GrabComponent.OnDropped` _array_element (delegate `OnDropped_Event`)))
    (`self.DecreaseCellSize`)))

(fn `DecreaseCellSize`
  (`SceneComponent.SetWorldScale3D` (`self.Bolsa`) (`self.InitialCellScale`)))

(fn `IncreaseCellSize`
  (`SceneComponent.SetWorldScale3D` (`self.Bolsa`) (* (`self.InitialCellScale`) 1.2)))

(fn `TryCaptureObject`
  (params (GrabComponent :type "/Game/VRTemplate/Blueprints/GrabComponent Object Reference"))
  (`/Engine/EditorBlueprintResources/StandardMacros.IsValid` (`self.HeldActor`)
    (:`Is Not Valid`
      (bind _output_get (set `self.HeldActor` (`ActorComponent.GetOwner` GrabComponent)))
      (set `self.InitialActorScale` (`self.GetActorScale3D` _output_get))
      (`/Game/VRTemplate/Blueprints/GrabComponent.SetPrimitiveCompPhysics` GrabComponent false)
      (`self.K2_AttachToComponent` _output_get (`self.DefaultSceneRoot`) "None" "SnapToTarget" "KeepWorld" "KeepWorld" true)
      (`self.SetActorScale3D` (`self.HeldActor`) (* (`self.InitialCellScale`) 0.4)))))

(fn `TryDropObject`
  (params (Actor :type "Actor Object Reference"))
  (bind _heldactor (`self.HeldActor`))
  (`/Engine/EditorBlueprintResources/StandardMacros.IsValid` _heldactor
    (:`Is Valid`
      (if (== Actor _heldactor)
        (if (== (`self.GetAttachParentActor` (`self.HeldActor`)) self)
          (`self.K2_DetachFromActor` (`self.HeldActor`) "KeepWorld" "KeepWorld" "KeepWorld"))
        (`self.SetActorScale3D` (`self.HeldActor`) (`self.InitialActorScale`))
        (set `self.HeldActor` null)))))

(fn `UserConstructionScript`)