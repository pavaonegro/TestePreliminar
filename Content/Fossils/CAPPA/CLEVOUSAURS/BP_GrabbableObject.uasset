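; BP_GrabbableObject is a fossil exhibit actor with a touch-style VR button that toggles a fossil sprite.
; At BeginPlay it binds ShowInfo to the XRInteractive widget's button.
; VR pawn overlap with the Box simulates a click, dims the button and plays a sound; any end overlap restores opacity.
; ShowInfo flips FossilSprite visibility, propagating to children only when showing.
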(event `self.ReceiveBeginPlay`
  (`XR_InteractiveComponent.BindFunctionToButton` (`self.XR_Interactive`) self "ShowInfo" true))

(event `self.Box.OnComponentBeginOverlap`
  (params (OverlappedComponent :type "PrimitiveComponent Object Reference") (OtherActor :type "Actor Object Reference") (OtherComp :type "PrimitiveComponent Object Reference") (OtherBodyIndex :type Integer) (bFromSweep :type Boolean) (SweepResult :type "HitResult Structure (by ref)"))
  (cast `/Game/VRTemplate/Blueprints/VRPawn_New` OtherActor)
  (bind _asw_interactive_button (cast `W_InteractiveButton` (`WidgetComponent.GetWidget` (`self.XR_Interactive`))))
  (`W_InteractiveButton.OnButtonClicked` _asw_interactive_button)
  (`Widget.SetRenderOpacity` _asw_interactive_button 0.7)
  (`GameplayStatics.PlaySound2D` "/Game/SOUNDS/Click2w.Click2w" 1.0 1.0 0.0 null null))

(event `self.Box.OnComponentEndOverlap`
  (params (OverlappedComponent :type "PrimitiveComponent Object Reference") (OtherActor :type "Actor Object Reference") (OtherComp :type "PrimitiveComponent Object Reference") (OtherBodyIndex :type Integer))
  (bind _asw_interactive_button (cast `W_InteractiveButton` (`WidgetComponent.GetWidget` (`self.XR_Interactive`))))
  (`Widget.SetRenderOpacity` _asw_interactive_button 1.0))

(fn `ShowInfo`
  (cast `W_InteractiveButton` (`WidgetComponent.GetWidget` (`self.XR_Interactive`)))
  (if (`SceneComponent.IsVisible` (`self.Fossil_Sprite`))
    (`SceneComponent.SetVisibility` (`self.Fossil_Sprite`) false false)
    (else
      (`SceneComponent.SetVisibility` (`self.Fossil_Sprite`) true true))))

(fn `UserConstructionScript`)