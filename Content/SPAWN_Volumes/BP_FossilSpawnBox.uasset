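; BP_FossilSpawnBox is a VR dig-spot volume that reveals a fossil after repeated geology hammer (MarteloGeo) hits.
; Each overlap plays right-hand haptics, a random hammer sound and rock particles while incrementing a counter.
; The fourth hit spawns a BP_BreakableRock carrying the Fossil class, stops the beep, leaves VRPawn_New's FossilsArray and calls OnFossilSpawned.
; FoundTIME appends the discovery timestamp to a hardcoded D: drive text file.
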(event `self.ReceiveBeginPlay`)

(event `self.Box.OnComponentBeginOverlap`
  (params (OverlappedComponent :type "PrimitiveComponent Object Reference") (OtherActor :type "Actor Object Reference") (OtherComp :type "PrimitiveComponent Object Reference") (OtherBodyIndex :type Integer) (bFromSweep :type Boolean) (SweepResult :type "HitResult Structure (by ref)"))
  (bind _returnvalue (`SceneComponent.K2_GetComponentLocation` (`self.Box`)))
  (castclass `/Game/VRTemplate/Blueprints/MarteloGeo` (`GameplayStatics.GetObjectClass` OtherActor))
  (if true
    (`PlayerController.PlayHapticEffect` (`PlayerState.GetPlayerController` (`GameplayStatics.GetPlayerState` 0)) "/Game/VRTemplate/Haptics/MArtelo.MArtelo" "Right" 1.0 false)
    (`GameplayStatics.PlaySoundAtLocation` (`KismetArrayLibrary.Array_Random` (`self.Hammer_sounds`)) _returnvalue (struct) 1.0 1.0 0.0 null null null null)
    (`NiagaraFunctionLibrary.SpawnSystemAtLocation` "/Game/PARTICLES/ROCKS_particleNiagaraSystem.ROCKS_particleNiagaraSystem" (+ (`SceneComponent.K2_GetComponentLocation` (`self.Box`)) (-20.0 -30.0 0.0) (0.0 0.0 0.0)) (struct :`Roll` -30.0))
    (bind _result (`/Engine/EditorBlueprintResources/StandardMacros.IncrementInt` (`self.OverlapCounter`))
      (:`  `
        (set `self.OverlapCounter` _result)
        (if (== (`self.OverlapCounter`) 4)
          (`/Engine/EditorBlueprintResources/StandardMacros.DoOnce` false
            (:`Completed`
              (`|SpawnActorFromClass` "/Game/Rocks_fracture/BP_BreakableRock.BP_BreakableRock_C" (`KismetMathLibrary.Conv_VectorToTransform` (+ _returnvalue (0.0 10.0 100.0) (0.0 0.0 0.0))) "AdjustIfPossibleButAlwaysSpawn" "OverrideRootScale" null (`self.Fossil`) null)
              (`self.FoundTIME`)
              (`AudioComponent.Stop` (`self.Beep_Editado_Cue`))
              (set `self.isPlayingSound` false)
              (bind _returnvalue_2 (`GameplayStatics.GetActorOfClass` "/Game/VRTemplate/Blueprints/VRPawn_New.VRPawn_New_C"))
              (`/Engine/EditorBlueprintResources/StandardMacros.IsValid` _returnvalue_2
                (:`Is Valid`
                  (`KismetArrayLibrary.Array_RemoveItem` (`/Game/VRTemplate/Blueprints/VRPawn_New.Fossils_Array` _returnvalue_2) self)
                  (set `self.IsSpawned` true)
                  (`self.OnFossilSpawned`)))))
          (else
            (`KismetSystemLibrary.PrintString` "NOT ENOUGH")))))))

(fn `FoundTIME`
  (`KismetArrayLibrary.Array_Add` (`self.TimeFound`) (`KismetMathLibrary.Now`))
  (for _array_element (`self.TimeFound`)
    (bind (_year _month _day _hour _minute _second _millisecond) (`KismetMathLibrary.BreakDateTime` _array_element))
    (set `self.FoundTimeString` (`KismetStringLibrary.Concat_StrStr` (`self.FoundTimeString`) (`KismetStringLibrary.Concat_StrStr` "Found " (`KismetSystemLibrary.GetClassDisplayName` (`self.Fossil`)) (`KismetStringLibrary.Conv_IntToString` _hour) ":" (`KismetStringLibrary.Conv_IntToString` _minute) ":" (`KismetStringLibrary.Conv_IntToString` _second) ":" (`KismetStringLibrary.Conv_IntToString` _millisecond) " \n"))))
  (`FileSDKBPLibrary.WriteStringToFile` (`KismetStringLibrary.Concat_StrStr` "D:\\FOUND_TIME" "_" ".txt") (`self.FoundTimeString`) true))

(fn `UserConstructionScript`)