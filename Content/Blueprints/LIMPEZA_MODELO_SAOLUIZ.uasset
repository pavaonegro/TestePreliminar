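; Hammer-breaking interaction actor, apparently for cleaning a São Luiz fossil model, that yields a Clevosaurus grabbable via a breakable rock.
; Component hits from MarteloGeo trigger right-hand haptics, play a collapse sound at the impact point and increment a hit counter.
; On exactly the third hit it spawns BP_BreakableRock offset from the impact, passing BP_Clevosaurus_Grab as its GrabbableToSpawn; other hits print a debug message.
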(event `self.StaticMesh.OnComponentHit`
  (params (HitComponent :type "PrimitiveComponent Object Reference") (OtherActor :type "Actor Object Reference") (OtherComp :type "PrimitiveComponent Object Reference") (NormalImpulse :type "Vector Structure") (Hit :type "HitResult Structure (by ref)"))
  (castclass `/Game/VRTemplate/Blueprints/MarteloGeo` (`GameplayStatics.GetObjectClass` OtherActor))
  (if true
    (bind _output_get (set `self.Hit_Location` (`.Location` (`GameplayStatics.BreakHitResult` Hit))))
    (`PlayerController.PlayHapticEffect` (`GameplayStatics.GetPlayerController` 0) "/Game/VRTemplate/Haptics/MArtelo.MArtelo" "Right" 10000.0 false)
    (`GameplayStatics.PlaySoundAtLocation` "/Game/StarterContent/Audio/Collapse01.Collapse01" _output_get (struct) 1.0 1.0 0.0 null null null null)
    (bind _result (`/Engine/EditorBlueprintResources/StandardMacros.IncrementInt` (`self.OverlapCounter`))
      (:`  `
        (set `self.OverlapCounter` _result)
        (if (== (`self.OverlapCounter`) 3)
          (`|SpawnActorFromClass` "/Game/Rocks_fracture/BP_BreakableRock.BP_BreakableRock_C" (`KismetMathLibrary.Conv_VectorToTransform` (+ _output_get (100.0 -180.0 180.0))) "AdjustIfPossibleButAlwaysSpawn" "OverrideRootScale" null "/Game/Fossils/CAPPA/CLEVOUSAURS/BP_Clevosaurus_Grab.BP_Clevosaurus_Grab_C" null "/Game/Fossils/CAPPA/CLEVOUSAURS/BP_Clevosaurus_Grab.BP_Clevosaurus_Grab_C" "/Game/Fossils/CAPPA/CLEVOUSAURS/BP_Clevosaurus_Grab.BP_Clevosaurus_Grab_C")
          (else
            (`KismetSystemLibrary.PrintString` "NOT ENOUGH")))))))

(fn `UserConstructionScript`)